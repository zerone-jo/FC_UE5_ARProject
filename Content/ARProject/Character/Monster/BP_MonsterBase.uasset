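; Base monster character Blueprint that handles a floating health bar, hit reaction, death and pickup drop.
; Status HP changes update the floating HP widget, then call the empty HitAnimation function or, at zero health, OnDead.
; Death plays a zombie dying montage, unpossesses, and drives a timeline dissolve on dynamic copies of all mesh materials.
; When the dissolve finishes, it spawns the pickup from the data table row matching CharacterKey and destroys itself.
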(event `self.ReceiveBeginPlay`
  (`parent.ReceiveBeginPlay`)
  (bind _aswb_floating_hp (cast `/Game/ARProject/UI/WB_FloatingHP` (`WidgetComponent.GetWidget` (`self.HpBar`))))
  (bind _output_get (set `self.As WB Floating HP` _aswb_floating_hp))
  (`/Game/ARProject/UI/WB_FloatingHP.SetHpRate` _output_get 1.0)
  (add `BaseCharacterStatus.HPChanged` (`self.GetStatus`) (delegate `HPUIChanged`)))

(event `HPUIChanged`
  (params (hpRate :type "Float (single-precision)"))
  (bind (__health_basevalue __health_currentvalue) (break `GameplayAttributeData` (`BaseCharacterStatus._health` (`self.GetStatus`))))
  (`/Game/ARProject/UI/WB_FloatingHP.SetHpRate` (`self.As WB Floating HP`) hpRate)
  (if (<= __health_currentvalue 0.0)
    (`self.OnDead`)
    (else
      (`self.HitAnimation`))))

(event `OnDead`
  (bind _mesh (`self.Mesh`))
  (`self.PlayAnimMontage` "/Game/ARProject/Character/Monster/SkeletonWarrior/Animations/Zombie_Dying_Montage.Zombie_Dying_Montage")
  (`Controller.UnPossess` (`self.GetController`))
  (`KismetArrayLibrary.Array_Clear` (`self.DynamicMaterials`))
  (for (_array_element _array_index) (`MeshComponent.GetMaterials` _mesh)
    (bind _returnvalue (`PrimitiveComponent.CreateDynamicMaterialInstance` _mesh _array_index _array_element "None"))
    (`KismetArrayLibrary.Array_Add` (`self.DynamicMaterials`) _returnvalue))
  (bind (_direction _dissolveamount) (`Timeline|DeadTimeLine` :!via `PlayFromStart`)
    (:`Update`
      (for _array_element_2 (`self.DynamicMaterials`)
        (`MaterialInstanceDynamic.SetScalarParameterValue` _array_element_2 "Dissolve" _dissolveamount)))
    (:`Finished`
      (`self.DropPickup`)
      (`self.K2_DestroyActor`))))

(fn `DropPickup`
  (bind _returnvalue (`|GetDataTableRow` (`self._pickupTable`) (`self._characterKey`))
    (:`then`
      (`|SpawnActorFromClass` (`._pickup` (break `PickupStaticData` _returnvalue)) (`self.GetTransform`) "AlwaysSpawn" "MultiplyWithRoot" null null))))

(fn `HitAnimation`)

(fn `UserConstructionScript`
  (`parent.UserConstructionScript`))