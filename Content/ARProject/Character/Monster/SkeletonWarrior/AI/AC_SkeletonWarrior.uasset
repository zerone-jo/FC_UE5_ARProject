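; AI controller for the Skeleton Warrior monster that runs its behavior tree on possess.
; Perception updates write a sensed Player-tagged actor to the blackboard as the target, flag it in sight and cancel any pending reset.
; Any other update, including lost sight or non-player actors, starts a two-second timer that clears the flag and target, giving a short grace period before forgetting the player.
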(event `self.ReceivePossess`
  (params (PossessedPawn :type "Pawn Object Reference"))
  (`self.RunBehaviorTree` "/Game/ARProject/Character/Monster/SkeletonWarrior/AI/BT_MonsterSkeletonWarrior.BT_MonsterSkeletonWarrior"))

(event `self.AIPerception.OnTargetPerceptionUpdated`
  (params (Actor :type "Actor Object Reference") (Stimulus :type "AIStimulus Structure"))
  (bind _blackboard (`self.Blackboard`))
  (if (and (`self.ActorHasTag` Actor "Player") (`.bSuccessfullySensed` (break `AIStimulus` Stimulus)))
    (`KismetSystemLibrary.K2_ClearAndInvalidateTimerHandle` (`self.ResetTimer`))
    (`BlackboardComponent.SetValueAsBool` _blackboard (`self.IsInSight`) true)
    (`BlackboardComponent.SetValueAsObject` _blackboard (`self.TargetActor`) Actor)
    (else
      (bind _returnvalue (`KismetSystemLibrary.K2_SetTimerDelegate` (delegate `ResetSight`) 2.0))
      (set `self.ResetTimer` _returnvalue))))

(event `ResetSight`
  (bind _blackboard (`self.Blackboard`))
  (`BlackboardComponent.SetValueAsBool` _blackboard (`self.IsInSight`) false)
  (`BlackboardComponent.SetValueAsObject` _blackboard (`self.TargetActor`) null))

(fn `UserConstructionScript`)