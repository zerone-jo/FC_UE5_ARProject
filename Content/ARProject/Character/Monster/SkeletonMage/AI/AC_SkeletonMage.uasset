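; AI controller for the Skeleton Mage monster that runs its behavior tree on possession and tracks the player through AI perception.
; A successfully sensed actor tagged Player cancels the reset timer and is written to the blackboard as the in-sight target.
; Any other perception update starts a short timer that clears the sight flag and target, so losing the player takes effect after a delay.
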(event `self.ReceivePossess`
  (params (PossessedPawn :type "Pawn Object Reference"))
  (`self.RunBehaviorTree` "/Game/ARProject/Character/Monster/SkeletonMage/AI/BT_MonsterSkeletonMage.BT_MonsterSkeletonMage"))

(event `ResetSight`
  (bind _blackboard (`self.Blackboard`))
  (`BlackboardComponent.SetValueAsBool` _blackboard (`self.IsInSight`) false)
  (`BlackboardComponent.SetValueAsObject` _blackboard (`self.TargetActor`) null))

(event `self.AIPerception.OnTargetPerceptionUpdated`
  (params (Actor :type "Actor Object Reference") (Stimulus :type "AIStimulus Structure"))
  (bind _blackboard (`self.Blackboard`))
  (if (and (`self.ActorHasTag` Actor "Player") (`.bSuccessfullySensed` (break `AIStimulus` Stimulus)))
    (`KismetSystemLibrary.K2_ClearAndInvalidateTimerHandle` (`self.ResetTimer`))
    (`BlackboardComponent.SetValueAsBool` _blackboard (`self.IsInSight`) true)
    (`BlackboardComponent.SetValueAsObject` _blackboard (`self.TargetActor`) Actor)
    (else
      (bind _returnvalue (`KismetSystemLibrary.K2_SetTimerDelegate` (delegate `ResetSight`) 2.0))
      (set `self.ResetTimer` _returnvalue))))

(fn `UserConstructionScript`)