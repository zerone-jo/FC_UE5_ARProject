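; GA_BasicAttack is a gameplay ability for a character's basic attack, playing the GreatAttack1 montage and dealing damage.
; After committing, it plays the montage directly on the BaseCharacter mesh and listens for Ability.Skill.BasicAttack gameplay events.
; Each event applies DamageEffect to the payload's target, passing DamageRate as a SetByCaller magnitude.
; The ability ends when the montage completes or is interrupted; a PlayMontageAndWait task remains unconnected.
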(event `self.K2_ActivateAbility`
  (bind _returnvalue_owneractor (break `GameplayAbilityActorInfo` (`self.GetActorInfo`)))
  (bind _returnvalue (`self.K2_CommitAbility`))
  (if _returnvalue
    (bind _asbase_character (cast `BaseCharacter` _returnvalue_owneractor))
    (bind _output_get (set `self.As Base Character` _asbase_character))
    (`|PlayMontage` (`Character.Mesh` _output_get) "/Game/ARProject/Character/Player/Animations/GreatSwrod/GreatAttack1.GreatAttack1"
      (:`then`
        (bind (_asynctaskproxy _payload) (`AbilityTask_WaitGameplayEvent.WaitGameplayEvent` (struct :`TagName` "Ability.Skill.BasicAttack") null)
          (:`EventReceived`
            (bind _returnvalue_2 (`AbilitySystemBlueprintLibrary.AssignTagSetByCallerMagnitude` (`self.MakeOutgoingGameplayEffectSpec` (`self._damageEffect`)) (struct :`TagName` "Attack.DamageRate") (`self._damageRate`)))
            (`AbilitySystemComponent.BP_ApplyGameplayEffectSpecToTarget` (`self.GetAbilitySystemComponentFromActorInfo`) _returnvalue_2 (`AbilitySystemBlueprintLibrary.GetAbilitySystemComponent` (`.Target` (break `GameplayEventData` _payload)))))))
      (:`OnCompleted`
        (`self.K2_EndAbility` :!label _label))
      (:`OnInterrupted`
        (goto _label)))
    (else
      (`self.K2_EndAbility`))))