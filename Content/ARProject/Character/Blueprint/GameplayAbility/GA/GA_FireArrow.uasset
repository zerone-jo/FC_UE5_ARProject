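; Gameplay Ability that fires an arrow from the player's bow.
; After committing, it clears the aim trajectory, plays the shoot montage and waits for the FireArrow gameplay event.
; That event spawns BP_Arrow at the bow with the player's projectile velocity, gravity and a damage effect spec carrying a SetByCaller damage rate.
; Blend-out plays the unequip montage before ending and resetting bow flags, while interruption or cancellation ends immediately.
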(event `self.K2_ActivateAbility`
  (bind _returnvalue_owneractor (break `GameplayAbilityActorInfo` (`self.GetActorInfo`)))
  (bind _as_bp_player (`self.As BP Player`))
  (bind _returnvalue (`self.K2_CommitAbility`))
  (if _returnvalue
    (bind _asbp_player (cast `/Game/ARProject/Character/Player/BP_Player` _returnvalue_owneractor))
    (bind _output_get (set `self.As BP Player` _asbp_player))
    (set `/Game/ARProject/Character/Player/BP_Player.IsBowAttaking` true _output_get)
    (`BaseCharacter.ClearTrajectory` _output_get)
    (`AbilityTask_PlayMontageAndWait.CreatePlayMontageAndWaitProxy` "None" "/Game/ARProject/Character/Player/Animations/Bow/Bow_Shoot_Montage.Bow_Shoot_Montage"
      (:`then`
        (`AbilityTask_WaitGameplayEvent.WaitGameplayEvent` (struct :`TagName` "Ability.Skill.FireArrow") null
          (:`EventReceived`
            (bind _returnvalue_2 (`AbilitySystemBlueprintLibrary.AssignTagSetByCallerMagnitude` (`self.MakeOutgoingGameplayEffectSpec` (`self._damageEffect`)) (struct :`TagName` "Attack.DamageRate") (`self._damageRate`)))
            (bind _returnvalue_3 (`|SpawnActorFromClass` "/Game/ARProject/Character/Player/Bow/BP_Arrow.BP_Arrow_C" (`SceneComponent.K2_GetComponentToWorld` (`/Game/ARProject/Character/Player/BP_Player.Bow` (`self.As BP Player`))) "AlwaysSpawn" "MultiplyWithRoot" null null))
            (set `/Game/ARProject/Character/Player/Bow/BP_Arrow.DamageEffectSpec` _returnvalue_2 _returnvalue_3)
            (bind _projectilemovement (`/Game/Projectiles_Spells_VFX_Vol_2/Blueprints/BP_Projectile_Main.ProjectileMovement` _returnvalue_3))
            (set `MovementComponent.Velocity` (`BaseCharacter._projectileVelocity` (`self.As BP Player`)) _projectilemovement)
            (set `ProjectileMovementComponent.ProjectileGravityScale` 1.0 _projectilemovement))))
      (:`OnBlendOut`
        (`|PlayMontage` (`Character.Mesh` _as_bp_player) "/Game/ARProject/Character/Player/Animations/Bow/Bow_UnEquip_Montage.Bow_UnEquip_Montage"
          (:`OnCompleted`
            (`self.K2_EndAbility` :!label _label)
            (set `/Game/ARProject/Character/Player/BP_Player.IsBow` false _as_bp_player)
            (set `/Game/ARProject/Character/Player/BP_Player.IsBowAttaking` false _as_bp_player))))
      (:`OnInterrupted`
        (goto _label))
      (:`OnCancelled`
        (goto _label)))
    (else
      (`self.K2_EndAbility`))))