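; BP_BaseCharacter is a base character Blueprint that supplies a shared ranged attack and placeholder weapon location queries.
; RangeAttack spawns a given projectile class at the GetMuzzle location, rotated to face the target actor's location, ignoring collisions at spawn.
; GetMuzzle, GetWeaponTop and GetWeaponBottom return zero vectors here, apparently as stubs for child Blueprints to override.
; The event graph and construction script contain no logic.
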(fn `GetMuzzle`
  (returns (Position :type "Vector Structure"))
  (return (0.0 0.0 0.0)))

(fn `GetWeaponBottom`
  (returns (Position :type "Vector Structure"))
  (return (0.0 0.0 0.0)))

(fn `GetWeaponTop`
  (returns (Position :type "Vector Structure"))
  (return (0.0 0.0 0.0)))

(fn `RangeAttack`
  (params (Projectile :type "/Game/Projectiles_Spells_VFX_Vol_2/Blueprints/BP_Projectile_Main Class Reference") (Target :type "/Game/ARProject/Character/Blueprint/Character/BP_BaseCharacter Object Reference"))
  (bind _position (`self.GetMuzzle`))
  (`|SpawnActorFromClass` Projectile (`KismetMathLibrary.MakeTransform` _position (`KismetMathLibrary.FindLookAtRotation` _position (`self.K2_GetActorLocation` Target))) "AlwaysSpawn" "MultiplyWithRoot" null null))

(fn `UserConstructionScript`)