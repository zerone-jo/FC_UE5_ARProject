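; BP_Arrow is the bow arrow actor that damages monsters it overlaps, using the Gameplay Ability System.
; On overlap with a BP_MonsterBase, it reads the instigator from the context of its DamageEffectSpec handle.
; The instigator's ability system component then applies that spec to the monster's component.
; The graph contains no movement logic and does not destroy the arrow after a hit.
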(event `self.ReceiveActorBeginOverlap`
  (params (OtherActor :type "Actor Object Reference"))
  (bind _damageeffectspec (`self.DamageEffectSpec`))
  (bind _asbp_monster_base (cast `/Game/ARProject/Character/Monster/BP_MonsterBase` OtherActor))
  (bind _returnvalue (`AbilitySystemBlueprintLibrary.GetEffectContext` _damageeffectspec))
  (`AbilitySystemComponent.BP_ApplyGameplayEffectSpecToTarget` (`AbilitySystemBlueprintLibrary.GetAbilitySystemComponent` (`AbilitySystemBlueprintLibrary.EffectContextGetInstigatorActor` _returnvalue)) _damageeffectspec (`AbilitySystemBlueprintLibrary.GetAbilitySystemComponent` _asbp_monster_base)))

(fn `UserConstructionScript`
  (`parent.UserConstructionScript`))